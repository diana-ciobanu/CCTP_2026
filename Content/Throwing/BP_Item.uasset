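; BP_Item is a throwable item with a configurable mesh that makes noise on impact.
; When the player is not holding an item, hits above a mass-scaled impulse threshold and outside a cooldown play an explosion effect and sound.
; Each hit calls Propagation on the game mode's sound system, with low, mid and high band intensities derived from kinetic energy and the player as instigator.
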(event OnComponentHit(ItemModel)
  (params (HitComponent :type Primitive%20Component%20Object%20Reference) (OtherActor :type Actor%20Object%20Reference) (OtherComp :type Primitive%20Component%20Object%20Reference) (NormalImpulse :type Vector :default "0, 0, 0") (Hit :type Hit%20Result%20Structure%20%28by%20ref%29))
  (bind _returnvalue (+ (.location Hit) "0.000000,0.000000,10.000000"))
  (bind _item_model (Variables|Default|GetItem%20Model))
  (bind _noisescale (Variables|Default|GetNoiseScale))
  (bind _returnvalue_2 (Physics|GetMass _item_model))
  (bind _returnvalue_3 (Transformation|GetComponentVelocity _item_model))
  (bind _returnvalue_4 (Math|Vector|VectorLength _returnvalue_3))
  (bind _returnvalue_5 (/ _returnvalue_4 1e+02))
  (bind _returnvalue_6 (Math|Float|Square _returnvalue_5))
  (bind _returnvalue_7 (* _returnvalue_2 _returnvalue_6 _noisescale 0.5))
  (bind _asbp_first_person_character (Utilities|Casting|CastToBP_FirstPersonCharacter (Game|Player|GetPlayerPawn 0)))
  (if (and (and (== (Variables|/Game/FirstPerson/Blueprints/BP_FirstPersonCharacter.BP_FirstPersonCharacter_C|GetHolding%20Item _asbp_first_person_character) false) (> (Math|Vector|VectorLength NormalImpulse) (* (Physics|GetMass (Variables|Default|GetItem%20Model)) 1e+02))) (>= (- (Utilities|Time|GetGameTimeinSeconds) (Variables|Default|GetLastHitTime)) (Variables|Default|GetHitCooldown)))
    (Variables|Default|SetLastHitTime (Utilities|Time|GetGameTimeinSeconds))
    (Effects|SpawnEmitteratLocation "/Game/StarterContent/Particles/P_Explosion.P_Explosion" _returnvalue)
    (Audio|PlaySoundatLocation "/Game/StarterContent/Audio/Explosion_Cue.Explosion_Cue" _returnvalue "0, 0, 0" 1.0 1.0 0.0 0 0 0 0)
    (Development|PrintString (Utilities|String|Append (Utilities|String|ToString(Float) _returnvalue_2) "   " (Utilities|String|ToString(Float) _returnvalue_5)))
    (Default|Propagation (Variables|Default|GetLocalItemSoundSystemRef) _returnvalue self (* _returnvalue_7 1.8) (* _returnvalue_7 0.9) (* _returnvalue_7 0.6) "/Game/StarterContent/Audio/Explosion_Cue.Explosion_Cue" _asbp_first_person_character)))

(event EventBeginPlay
  (Utilities|FlowControl|DelayUntilNextTick)
  (bind _asbp_custom_game_mode (Utilities|Casting|CastToBP_CustomGameMode (Game|GetGameMode)))
  (Variables|Default|SetLocalItemSoundSystemRef (Variables|/Game/FirstPerson/Blueprints/BP_CustomGameMode.BP_CustomGameMode_C|GetSoundSystemRef _asbp_custom_game_mode)))

(fn ConstructionScript
  (Components|StaticMesh|SetStaticMesh (Variables|Default|GetItem%20Model) (Variables|Default|GetItemModelToPlace)))