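; Base enemy character driven by AIC_Enemy_Base, with a punch montage attack, patrol route getter and enum-based walk speed setter.
; Hearing is simulated physically: BP_DebugSphere overlaps on the Hearing component add sound intensity and record the origin, while a looping timer halves the total.
; Tick sends the controller to investigate that origin when intensity passes a threshold in the initial enum state, then resets it.
; Attack end is broadcast on completion or interruption.
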(event OnComponentBeginOverlap(Hearing)
  (params (OverlappedComponent :type Primitive%20Component%20Object%20Reference) (OtherActor :type Actor%20Object%20Reference) (OtherComp :type Primitive%20Component%20Object%20Reference) (OtherBodyIndex :type Integer) (bFromSweep :type Boolean) (SweepResult :type Hit%20Result%20Structure%20%28by%20ref%29))
  (bind _asbp_debug_sphere (Utilities|Casting|CastToBP_DebugSphere OtherActor))
  (Variables|Default|SetAccumulatedIntensity (+ (Variables|/Game/SoundSystem/BP_DebugSphere.BP_DebugSphere_C|GetCurrentIntensity _asbp_debug_sphere) (Variables|Default|GetAccumulatedIntensity)))
  (Variables|Default|SetSoundLocation (Variables|/Game/SoundSystem/BP_DebugSphere.BP_DebugSphere_C|GetStartPos _asbp_debug_sphere))
  (Development|PrintString (Utilities|String|ToString(Float) (Variables|Default|GetAccumulatedIntensity))))

(event Custom|HearSound
  (params (Location :type Vector))
  (bind _asaic_enemy_base (Utilities|Casting|CastToAIC_Enemy_Base (Pawn|GetController)))
  (Default|SetStateInvestigating _asaic_enemy_base Location))

(event Custom|Attack
  (Animation|Montage|PlayMontage (Variables|Character|GetMesh) "/Game/Enemies/Animations/Montage_Enemy_CrossPunch.Montage_Enemy_CrossPunch"
    (:OnCompleted
      _)
    (:OnInterrupted
      _))
  (Default|CallOnAttackEnd))

(event Custom|LoseIntensity
  (Variables|Default|SetAccumulatedIntensity (* (Variables|Default|GetAccumulatedIntensity) 0.5)))

(event EventBeginPlay
  (bind _asaic_enemy_base (Utilities|Casting|CastToAIC_Enemy_Base (Pawn|GetController)))
  (Variables|Default|SetAIC%20Enemy%20Base _asaic_enemy_base)
  (Utilities|Time|SetTimerbyEvent (delegate Custom|LoseIntensity) 5.0 true))

(event EventTick
  (params (DeltaSeconds :type Float%20%28single-precision%29))
  (bind _state (Default|GetCurrentState (Variables|Default|GetAIC%20Enemy%20Base)))
  (if (and (> (Variables|Default|GetAccumulatedIntensity) (Variables|Default|GetIntensityThreshold)) (== _state 0))
    (CallFunction|HearSound (Variables|Default|GetSoundLocation))
    (Variables|Default|SetAccumulatedIntensity 0.0)))

(fn ConstructionScript)

(fn GetPatrolRoute
  (return (Variables|AI|GetPatrolRoute)))

(fn SetMovementSpeed
  (params (Speed :type E_Movespeed%20Enum :default "NewEnumerator0"))
  (bind _output_get (Variables|/Script/Engine.CharacterMovementComponent|SetMaxWalkSpeed (Variables|Character|GetCharacterMovement) (Utilities|Select :Index Speed :NewEnumerator0 0.0 :NewEnumerator1 1e+02 :NewEnumerator2 3e+02 :NewEnumerator3 5e+02)))
  (return _output_get))