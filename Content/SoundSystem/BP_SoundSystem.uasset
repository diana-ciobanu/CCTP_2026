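; BP_SoundSystem simulates sound propagation under a selectable model, from simple linear to diffraction, materials and transmission, or Unreal's built-in noise perception.
; It registers with the game mode, casts a ray grid from each sound, optionally extends paths by reflection and precomputes transmission endpoints.
; Each path spawns a BP_DebugSphere packet carrying three-band intensities.
; Transmission and diffraction handlers spawn secondary packets with divided intensity.
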(event Custom|SetDefaultSettings
  (Utilities|Struct|SetmembersinS_SoundVariables (Variables|Default|GetDefaultSettings))
  (Variables|Default|SetCurrentSettings ""))

(event Custom|UnrealPerception
  (params (Location :type Vector) (Sound :type Sound%20Base%20Object%20Reference) (NoiseInstigator :type Pawn%20Object%20Reference))
  (Audio|PlaySoundatLocation Sound Location "0, 0, 0" 1.0 1.0 0.0 0 0 0 0)
  (Class|Actor|MakeNoise 1.0 NoiseInstigator Location 0.0 "None"))

(event Custom|ResetVariables
  (Utilities|Array|Clear (Variables|Default|GetAllRays))
  (Utilities|Array|Clear (Variables|Default|GetSoundPath))
  (Utilities|Array|Clear (Variables|Default|GetTransmissionPath)))

(event Custom|Reverb
  (if (Variables|Default|GetCanReflect)
    (for (_ _array_index) (Variables|Default|GetAllRays)
      (for _index (range 0 (- (.imax_bounces (Variables|Default|GetCurrentSettings)) 1))
        (bind _outhit (Collision|LineTraceByChannel (+ (.pathlocations (Utilities|Array|Get(acopy) (.path (Utilities|Array|Get(acopy) (Variables|Default|GetAllRays) _array_index)) (Utilities|Array|LastIndex (.path (Utilities|Array|Get(acopy) (Variables|Default|GetAllRays) _array_index))))) (* (.pathnormals (Utilities|Array|Get(acopy) (.path (Utilities|Array|Get(acopy) (Variables|Default|GetAllRays) _array_index)) (Utilities|Array|LastIndex (.path (Utilities|Array|Get(acopy) (Variables|Default|GetAllRays) _array_index))))) 5)) (+ (+ (.pathlocations (Utilities|Array|Get(acopy) (.path (Utilities|Array|Get(acopy) (Variables|Default|GetAllRays) _array_index)) (Utilities|Array|LastIndex (.path (Utilities|Array|Get(acopy) (Variables|Default|GetAllRays) _array_index))))) (* (.pathnormals (Utilities|Array|Get(acopy) (.path (Utilities|Array|Get(acopy) (Variables|Default|GetAllRays) _array_index)) (Utilities|Array|LastIndex (.path (Utilities|Array|Get(acopy) (Variables|Default|GetAllRays) _array_index))))) 5)) (* (Math|Vector|GetReflectionVector (Math|Vector|Normalize (- (.pathlocations (Utilities|Array|Get(acopy) (.path (Utilities|Array|Get(acopy) (Variables|Default|GetAllRays) _array_index)) (Utilities|Array|LastIndex (.path (Utilities|Array|Get(acopy) (Variables|Default|GetAllRays) _array_index))))) (.pathlocations (Utilities|Array|Get(acopy) (.path (Utilities|Array|Get(acopy) (Variables|Default|GetAllRays) _array_index)) (- (Utilities|Array|LastIndex (.path (Utilities|Array|Get(acopy) (Variables|Default|GetAllRays) _array_index))) 1))))) (.pathnormals (Utilities|Array|Get(acopy) (.path (Utilities|Array|Get(acopy) (Variables|Default|GetAllRays) _array_index)) (Utilities|Array|LastIndex (.path (Utilities|Array|Get(acopy) (Variables|Default|GetAllRays) _array_index)))))) (Variables|Default|GetRayLength))) "TraceTypeQuery1" false 0 (Variables|Default|GetDraw%20Debug%20Type)))
        (if (.bblockinghit _outhit)
          (if (Variables|Default|GetCanUseMaterials)
            (Utilities|Array|Add (.path (Utilities|Array|Get(acopy) (Variables|Default|GetAllRays) _array_index)) (Utilities|Struct|MakeS_SoundPath (.impactpoint _outhit) (.impactnormal _outhit) (.Value (Utilities|Map|Find (Variables|Default|GetMaterialMap) (.physmat _outhit)))))
            (Utilities|Array|Add :TargetArray (Variables|Default|GetTransmissionPath))
            (else
              (Utilities|Array|Add (.path (Utilities|Array|Get(acopy) (Variables|Default|GetAllRays) _array_index)) (Utilities|Struct|MakeS_SoundPath (.impactpoint _outhit) (.impactnormal _outhit) (Variables|Default|GetDefaultMaterial)))
              (Utilities|Array|Add :TargetArray (Variables|Default|GetTransmissionPath)))))))))

(event Custom|PrintAHits
  (for (_array_element _array_index) (Variables|Default|GetAllRays)
    (for _array_element_2 (.path _array_element)
      (Development|PrintString (Utilities|String|Append "Direction" (Utilities|String|ToString(Integer) (.direction _array_element))))
      (Development|PrintString (Utilities|String|Append "Location" (Utilities|String|ToString(Vector) (.pathlocations _array_element_2))))
      (Development|PrintString (Utilities|String|Append "Normal" (Utilities|String|ToString(Vector) (.pathnormals _array_element_2)))))
    (Development|PrintString (Utilities|String|Append "Number of elements in SoundPath " (Utilities|String|ToString(Integer) (+ (Utilities|Array|LastIndex (Variables|Default|GetSoundPath)) 1)))))
  (Development|PrintString (Utilities|String|Append "Number of rays in AHits " (Utilities|String|ToString(Integer) (+ _array_index 1)))))

(event Custom|Transmission
  (if (Variables|Default|GetCanTransmit)
    (Utilities|Array|Clear (Variables|Default|GetTransmissionPath))
    (for _array_element (Variables|Default|GetAllRays)
      (Utilities|Array|Clear (.bounces (Variables|Default|GetTransmissionRay)))
      (for _index (range 1 (- (Utilities|Array|Length (.path _array_element)) 1))
        (Utilities|Array|Clear (.endpoints (Variables|Default|GetTransmissionBounce)))
        (Variables|Default|SetTransmissionNormal (.pathnormals (Utilities|Array|Get(acopy) (.path _array_element) _index)))
        (if (> (Math|Vector|DotProduct (Math|Vector|Normalize (- (.pathlocations (Utilities|Array|Get(acopy) (.path _array_element) _index)) (.pathlocations (Utilities|Array|Get(acopy) (.path _array_element) (- _index 1))))) (Variables|Default|GetTransmissionNormal)) 0.0)
          (Variables|Default|SetTransmissionNormal (* (Variables|Default|GetTransmissionNormal) -1)))
        (for _index_2 (range 0 (- (.itransmission_rays (Variables|Default|GetCurrentSettings)) 1))
          (Variables|Default|SetTransmissionDir (Math|Vector|Normalize (+ (* (Math|Random|RandomUnitVector) 0.9) (Math|Vector|Normalize (- (.pathlocations (Utilities|Array|Get(acopy) (.path _array_element) _index)) (.pathlocations (Utilities|Array|Get(acopy) (.path _array_element) (- _index 1))))))))
          (if (> (Math|Vector|DotProduct (Variables|Default|GetTransmissionDir) (Variables|Default|GetTransmissionNormal)) 0.0)
            (Variables|Default|SetTransmissionDir (* (Variables|Default|GetTransmissionDir) -1)))
          (Collision|LineTraceByChannel (.pathlocations (Utilities|Array|Get(acopy) (.path _array_element) _index)) (+ (.pathlocations (Utilities|Array|Get(acopy) (.path _array_element) _index)) (* 30 (Variables|Default|GetTransmissionDir))) "TraceTypeQuery1" false 0 (Variables|Default|GetDraw%20Debug%20Type) true "(R=0.000000,G=0.070871,B=1.000000,A=1.000000)" "(R=1.000000,G=0.071198,B=0.846682,A=1.000000)")
          (Utilities|Array|Add (.endpoints (Variables|Default|GetTransmissionBounce)) (+ (.pathlocations (Utilities|Array|Get(acopy) (.path _array_element) _index)) (* 30 (Variables|Default|GetTransmissionDir)))))
        (Utilities|Array|Add (.bounces (Variables|Default|GetTransmissionRay)) (Variables|Default|GetTransmissionBounce)))
      (Utilities|Array|Add (Variables|Default|GetTransmissionPath) (Variables|Default|GetTransmissionRay)))))

(event Custom|HandleTransmission
  (params (SphereIndex :type Integer) (BounceIndex :type Integer) (EndPos :type Vector) (LFIntensity :type Float%20%28double-precision%29) (MFIntensity :type Float%20%28double-precision%29) (HFIntensity :type Float%20%28double-precision%29))
  (bind _currentsettings (Variables|Default|GetCurrentSettings))
  (if (Variables|Default|GetCanTransmit)
    (for _array_element (.endpoints (Utilities|Array|Get(acopy) (.bounces (Utilities|Array|Get(acopy) (Variables|Default|GetTransmissionPath) SphereIndex)) (+ BounceIndex 0)))
      (Game|SpawnActorfromClass "/Game/SoundSystem/BP_DebugSphere.BP_DebugSphere_C" (Math|Transform|MakeTransform EndPos "0, 0, 0" "2.000000,2.000000,2.000000") "Undefined" "MultiplyWithRoot" 0 0 (Utilities|Struct|MakeS_SoundPacket true (Utilities|Array|MakeArray (Utilities|Struct|MakeS_SoundPath EndPos "0.000000,0.000000,0.000000" "(AbsorptionLF_19_582268854A432637AD5B97ADC9E1E34B=0.000000,AbsorptionMF_20_F3CE78F74C2024501FD6DAA60CC9747A=0.000000,AbsorptionHF_21_36D7B56B4E03BA28E52E18B3835A42DB=0.000000,TransmissionLF_12_8DB504DC47A61470FF477B949CB2C7C0=0.000000,TransmissionMF_13_5579781A4D36D0123777128C6EAAA77D=0.000000,TransmissionHF_14_BE344B8C49141F016D0818A0704C06BA=0.000000)") (Utilities|Struct|MakeS_SoundPath _array_element "0.000000,0.000000,0.000000" "(AbsorptionLF_19_582268854A432637AD5B97ADC9E1E34B=0.000000,AbsorptionMF_20_F3CE78F74C2024501FD6DAA60CC9747A=0.000000,AbsorptionHF_21_36D7B56B4E03BA28E52E18B3835A42DB=0.000000,TransmissionLF_12_8DB504DC47A61470FF477B949CB2C7C0=0.000000,TransmissionMF_13_5579781A4D36D0123777128C6EAAA77D=0.000000,TransmissionHF_14_BE344B8C49141F016D0818A0704C06BA=0.000000)")) 0 0.0 (Math|Conversions|ToFloat(Integer) (.ispeed (Variables|Default|GetCurrentSettings))) (/ LFIntensity (.itransmission_rays _currentsettings)) (/ MFIntensity (.itransmission_rays _currentsettings)) (/ HFIntensity (.itransmission_rays _currentsettings)) 0.0 false false "(AbsorptionLF_19_582268854A432637AD5B97ADC9E1E34B=0.000000,AbsorptionMF_20_F3CE78F74C2024501FD6DAA60CC9747A=0.000000,AbsorptionHF_21_36D7B56B4E03BA28E52E18B3835A42DB=0.000000,TransmissionLF_12_8DB504DC47A61470FF477B949CB2C7C0=0.000000,TransmissionMF_13_5579781A4D36D0123777128C6EAAA77D=0.000000,TransmissionHF_14_BE344B8C49141F016D0818A0704C06BA=0.000000)") 0))))

(event Custom|HandleDiffraction
  (params (ImpactPoint :type Vector) (Direction :type Vector) (Edge :type BP%20Diffraction%20Edge%20Object%20Reference) (LFIntensity :type Float%20%28double-precision%29) (MFIntensity :type Float%20%28double-precision%29) (HFIntensity :type Float%20%28double-precision%29))
  (bind _returnvalue (Math|Random|RandomUnitVector))
  (bind _returnvalue_2 (Math|Vector|Normalize Direction))
  (bind _currentsettings (Variables|Default|GetCurrentSettings))
  (bind _cube (Variables|/Game/SoundSystem/BP_DiffractionEdge.BP_DiffractionEdge_C|GetCube Edge))
  (bind _returnvalue_3 (Transformation|GetWorldLocation _cube))
  (bind _returnvalue_4 (* _returnvalue 0.3))
  (bind _returnvalue_5 (Math|Vector|MakeVector (.x _returnvalue_3) (.y _returnvalue_3) (.z ImpactPoint)))
  (bind _returnvalue_6 (+ _returnvalue_2 _returnvalue_4))
  (bind _returnvalue_7 (Math|Vector|Normalize _returnvalue_6))
  (if (Variables|Default|GetCanDiffract)
    (for _index (range 0 (- (.idiffraction_rays (Variables|Default|GetCurrentSettings)) 1))
      (Variables|Default|SetDiffractionDir _returnvalue_7)
      (if (< (Math|Vector|DotProduct _returnvalue_7 _returnvalue_2) 0.0)
        (Variables|Default|SetDiffractionDir (* (Variables|Default|GetDiffractionDir) -1)))
      (Collision|LineTraceByChannel _returnvalue_5 (+ (* (Variables|Default|GetDiffractionDir) (Variables|Default|GetRayLength)) _returnvalue_5) "TraceTypeQuery1" false 0 (Variables|Default|GetDraw%20Debug%20Type))
      (Game|SpawnActorfromClass "/Game/SoundSystem/BP_DebugSphere.BP_DebugSphere_C" (Math|Transform|MakeTransform _returnvalue_5 "0, 0, 0" "0.500000,0.500000,0.500000") "Undefined" "MultiplyWithRoot" 0 0 (Utilities|Struct|MakeS_SoundPacket false (Utilities|Array|MakeArray (Utilities|Struct|MakeS_SoundPath _returnvalue_5 "0.000000,0.000000,0.000000" "(AbsorptionLF_19_582268854A432637AD5B97ADC9E1E34B=0.000000,AbsorptionMF_20_F3CE78F74C2024501FD6DAA60CC9747A=0.000000,AbsorptionHF_21_36D7B56B4E03BA28E52E18B3835A42DB=0.000000,TransmissionLF_12_8DB504DC47A61470FF477B949CB2C7C0=0.000000,TransmissionMF_13_5579781A4D36D0123777128C6EAAA77D=0.000000,TransmissionHF_14_BE344B8C49141F016D0818A0704C06BA=0.000000)") (Utilities|Struct|MakeS_SoundPath (+ (* (Variables|Default|GetDiffractionDir) (Variables|Default|GetRayLength)) _returnvalue_5) "0.000000,0.000000,0.000000" "(AbsorptionLF_19_582268854A432637AD5B97ADC9E1E34B=0.000000,AbsorptionMF_20_F3CE78F74C2024501FD6DAA60CC9747A=0.000000,AbsorptionHF_21_36D7B56B4E03BA28E52E18B3835A42DB=0.000000,TransmissionLF_12_8DB504DC47A61470FF477B949CB2C7C0=0.000000,TransmissionMF_13_5579781A4D36D0123777128C6EAAA77D=0.000000,TransmissionHF_14_BE344B8C49141F016D0818A0704C06BA=0.000000)")) 0 0.0 (Math|Conversions|ToFloat(Integer) (.ispeed (Variables|Default|GetCurrentSettings))) (/ LFIntensity (.idiffraction_rays _currentsettings)) (/ MFIntensity (.idiffraction_rays _currentsettings)) (/ HFIntensity (.idiffraction_rays _currentsettings)) 0.0 false false "(AbsorptionLF_19_582268854A432637AD5B97ADC9E1E34B=0.000000,AbsorptionMF_20_F3CE78F74C2024501FD6DAA60CC9747A=0.000000,AbsorptionHF_21_36D7B56B4E03BA28E52E18B3835A42DB=0.000000,TransmissionLF_12_8DB504DC47A61470FF477B949CB2C7C0=0.000000,TransmissionMF_13_5579781A4D36D0123777128C6EAAA77D=0.000000,TransmissionHF_14_BE344B8C49141F016D0818A0704C06BA=0.000000)") 0))))

(event Custom|PrintActiveParticles
  (bind _outactors (Actor|GetAllActorsOfClass "/Game/SoundSystem/BP_DebugSphere.BP_DebugSphere_C"))
  (Development|PrintString (Utilities|String|ToString(Integer) (Utilities|Array|Length _outactors))))

(event Custom|ComplexDiffractionMaterialsTransmission
  (params (StartLocation :type Vector) (Emitter :type Actor%20Object%20Reference))
  (CallFunction|ResetVariables)
  (CallFunction|CastRays StartLocation Emitter)
  (CallFunction|Reverb)
  (CallFunction|Transmission)
  (CallFunction|SoundPackets))

(event Custom|SimpleLinearSound
  (params (StartLocation :type Vector) (Emitter :type Actor%20Object%20Reference))
  (CallFunction|ResetVariables)
  (CallFunction|CastRays StartLocation Emitter)
  (CallFunction|SoundPackets))

(event Custom|SimpleLinearReflectSound
  (params (StartLocation :type Vector) (Emitter :type Actor%20Object%20Reference))
  (CallFunction|ResetVariables)
  (CallFunction|CastRays StartLocation Emitter)
  (CallFunction|Reverb)
  (CallFunction|SoundPackets))

(event Custom|ComplexDiffractionSound
  (params (StartLocation :type Vector) (Emitter :type Actor%20Object%20Reference))
  (CallFunction|ResetVariables)
  (CallFunction|CastRays StartLocation Emitter)
  (CallFunction|Reverb)
  (CallFunction|Transmission)
  (CallFunction|SoundPackets))

(event Custom|ComplexDiffractionMaterialsSound
  (params (StartLocation :type Vector) (Emitter :type Actor%20Object%20Reference))
  (CallFunction|ResetVariables)
  (CallFunction|CastRays StartLocation Emitter)
  (CallFunction|Reverb)
  (CallFunction|Transmission)
  (CallFunction|SoundPackets))

(event Custom|CastRays
  (params (StartLocation :type Vector) (Emitter :type Actor%20Object%20Reference))
  (bind _soundpath (Variables|Default|GetSoundPath))
  (bind _currentsettings (Variables|Default|GetCurrentSettings))
  (bind _soundpath_2 (Variables|Default|GetSoundPath))
  (bind _returnvalue (- (.iray_count _currentsettings) 1))
  (for _index (range 0 _returnvalue)
    (for _index_2 (range 0 _returnvalue)
      (bind _outhit (Collision|LineTraceByChannel StartLocation (+ (* (Math|Vector|GetForwardVector (Math|Rotator|MakeRotator 0.0 (Math|Conversions|ToFloat(Integer) (* (/ 360 (.iray_count (Variables|Default|GetCurrentSettings))) _index_2)) (Math|Conversions|ToFloat(Integer) (* (/ 360 (.iray_count _currentsettings)) _index)))) (Variables|Default|GetRayLength)) StartLocation) "TraceTypeQuery1" false (Utilities|Array|MakeArray Emitter) (Variables|Default|GetDraw%20Debug%20Type) true "(R=0.000000,G=0.000000,B=0.000000,A=1.000000)" "(R=1.000000,G=1.000000,B=1.000000,A=1.000000)"))
      (if (Variables|Default|GetCanUseMaterials)
        (Utilities|Array|Add _soundpath_2 (Utilities|Struct|MakeS_SoundPath StartLocation "0.000000,0.000000,0.000000" "(AbsorptionLF_19_582268854A432637AD5B97ADC9E1E34B=0.000000,AbsorptionMF_20_F3CE78F74C2024501FD6DAA60CC9747A=0.000000,AbsorptionHF_21_36D7B56B4E03BA28E52E18B3835A42DB=0.000000,TransmissionLF_12_8DB504DC47A61470FF477B949CB2C7C0=0.000000,TransmissionMF_13_5579781A4D36D0123777128C6EAAA77D=0.000000,TransmissionHF_14_BE344B8C49141F016D0818A0704C06BA=0.000000)"))
        (Utilities|Array|Add _soundpath_2 (Utilities|Struct|MakeS_SoundPath (.impactpoint _outhit) (.impactnormal _outhit) (.Value (Utilities|Map|Find (Variables|Default|GetMaterialMap) (.physmat _outhit)))))
        (Utilities|Array|Add (Variables|Default|GetAllRays) (Utilities|Struct|MakeS_SoundHit (Math|Vector|Normalize (- (+ (* (Math|Vector|GetForwardVector (Math|Rotator|MakeRotator 0.0 (Math|Conversions|ToFloat(Integer) (* (/ 360 (.iray_count (Variables|Default|GetCurrentSettings))) _index_2)) (Math|Conversions|ToFloat(Integer) (* (/ 360 (.iray_count _currentsettings)) _index)))) (Variables|Default|GetRayLength)) StartLocation) StartLocation)) (.bblockinghit _outhit) (.distance _outhit) (Variables|Default|GetSoundPath) (.physmat _outhit) (.hitactor _outhit)))
        (Utilities|Array|Clear (Variables|Default|GetSoundPath))
        (else
          (Utilities|Array|Add _soundpath (Utilities|Struct|MakeS_SoundPath StartLocation "0.000000,0.000000,0.000000" "(AbsorptionLF_19_582268854A432637AD5B97ADC9E1E34B=0.000000,AbsorptionMF_20_F3CE78F74C2024501FD6DAA60CC9747A=0.000000,AbsorptionHF_21_36D7B56B4E03BA28E52E18B3835A42DB=0.000000,TransmissionLF_12_8DB504DC47A61470FF477B949CB2C7C0=0.000000,TransmissionMF_13_5579781A4D36D0123777128C6EAAA77D=0.000000,TransmissionHF_14_BE344B8C49141F016D0818A0704C06BA=0.000000)"))
          (Utilities|Array|Add _soundpath (Utilities|Struct|MakeS_SoundPath (.impactpoint _outhit) (.impactnormal _outhit) (Variables|Default|GetDefaultMaterial)))
          (Utilities|Array|Add (Variables|Default|GetAllRays) (Utilities|Struct|MakeS_SoundHit (Math|Vector|Normalize (- (+ (* (Math|Vector|GetForwardVector (Math|Rotator|MakeRotator 0.0 (Math|Conversions|ToFloat(Integer) (* (/ 360 (.iray_count (Variables|Default|GetCurrentSettings))) _index_2)) (Math|Conversions|ToFloat(Integer) (* (/ 360 (.iray_count _currentsettings)) _index)))) (Variables|Default|GetRayLength)) StartLocation) StartLocation)) (.bblockinghit _outhit) (.distance _outhit) (Variables|Default|GetSoundPath) (.physmat _outhit) (.hitactor _outhit)))
          (Utilities|Array|Clear (Variables|Default|GetSoundPath)))))))

(event Custom|Propagation
  (params (StartLocation :type Vector) (Emitter :type Actor%20Object%20Reference) (LFIntensity :type Float%20%28double-precision%29) (MFIntensity :type Float%20%28double-precision%29) (HFIntensity :type Float%20%28double-precision%29) (Sound :type Sound%20Base%20Object%20Reference) (NoiseInstigator :type Pawn%20Object%20Reference))
  (bind _currentsettings (Variables|Default|GetCurrentSettings))
  (bind (_bdebugvis _iray_count _imax_bounces _itransmission_rays _idiffraction_rays _ispeed _esound_models) (Utilities|Struct|BreakS_SoundVariables _currentsettings))
  (Variables|Default|SetLFIntensity LFIntensity)
  (Variables|Default|SetMFIntensity MFIntensity)
  (Variables|Default|SetHFIntensity HFIntensity)
  (if _bdebugvis
    (Variables|Default|SetDraw%20Debug%20Type "ForDuration"))
  (switch Utilities|FlowControl|Switch|SwitchonE_SoundModels _esound_models
    (:NewEnumerator0
      (CallFunction|SimpleLinearSound StartLocation Emitter)
      (Variables|Default|SetCanReflect false)
      (Variables|Default|SetCanTransmit false)
      (Variables|Default|SetCanDiffract false)
      (Variables|Default|SetCanUseMaterials true))
    (:NewEnumerator2
      (CallFunction|SimpleLinearReflectSound StartLocation Emitter)
      (Variables|Default|SetCanReflect true)
      (Variables|Default|SetCanTransmit false)
      (Variables|Default|SetCanDiffract false)
      (Variables|Default|SetCanUseMaterials true))
    (:NewEnumerator3
      (CallFunction|ComplexDiffractionSound StartLocation Emitter)
      (Variables|Default|SetCanReflect true)
      (Variables|Default|SetCanTransmit false)
      (Variables|Default|SetCanDiffract true)
      (Variables|Default|SetCanUseMaterials false))
    (:NewEnumerator4
      (CallFunction|ComplexDiffractionMaterialsSound StartLocation Emitter)
      (Variables|Default|SetCanReflect true)
      (Variables|Default|SetCanTransmit false)
      (Variables|Default|SetCanDiffract true)
      (Variables|Default|SetCanUseMaterials true))
    (:NewEnumerator5
      (CallFunction|ComplexDiffractionMaterialsTransmission StartLocation Emitter)
      (Variables|Default|SetCanReflect true)
      (Variables|Default|SetCanTransmit true)
      (Variables|Default|SetCanDiffract true)
      (Variables|Default|SetCanUseMaterials true))
    (:NewEnumerator6
      (CallFunction|UnrealPerception StartLocation Sound NoiseInstigator))))

(event Custom|SoundPackets
  (for (_array_element _array_index) (Variables|Default|GetAllRays)
    (Variables|Default|SetSphereIndex _array_index)
    (Game|SpawnActorfromClass "/Game/SoundSystem/BP_DebugSphere.BP_DebugSphere_C" (Math|Transform|MakeTransform (.pathlocations (Utilities|Array|Get(acopy) (.path _array_element))) "0, 0, 0" "1.000000,1.000000,1.000000") "Undefined" "MultiplyWithRoot" 0 self (Utilities|Struct|MakeS_SoundPacket true (.path _array_element) _array_index 0.0 (Math|Conversions|ToFloat(Integer) (.ispeed (Variables|Default|GetCurrentSettings))) (Variables|Default|GetLFIntensity) (Variables|Default|GetMFIntensity) (Variables|Default|GetHFIntensity) 0.0 true true "(AbsorptionLF_19_582268854A432637AD5B97ADC9E1E34B=0.000000,AbsorptionMF_20_F3CE78F74C2024501FD6DAA60CC9747A=0.000000,AbsorptionHF_21_36D7B56B4E03BA28E52E18B3835A42DB=0.000000,TransmissionLF_12_8DB504DC47A61470FF477B949CB2C7C0=0.000000,TransmissionMF_13_5579781A4D36D0123777128C6EAAA77D=0.000000,TransmissionHF_14_BE344B8C49141F016D0818A0704C06BA=0.000000)") 0)))

(event EventBeginPlay
  (bind _asbp_game_instance (Utilities|Casting|CastToBP_GameInstance (Game|GetGameInstance)))
  (bind _asbp_custom_game_mode (Utilities|Casting|CastToBP_CustomGameMode (Game|GetGameMode)))
  (Variables|/Game/FirstPerson/Blueprints/BP_CustomGameMode.BP_CustomGameMode_C|SetSoundSystemRef _asbp_custom_game_mode self)
  (Variables|Default|SetCurrentSettings (Variables|/Game/BP_GameInstance.BP_GameInstance_C|GetSoundSettings _asbp_game_instance))
  (Development|PrintText (Utilities|Text|ToText(Name) (Utilities|Name|EnumtoName (.esound_models (Variables|Default|GetCurrentSettings)))))
  (Utilities|Time|SetTimerbyEvent (delegate Custom|PrintActiveParticles) 2.0 true))

(fn ConstructionScript)