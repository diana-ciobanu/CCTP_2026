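; Debug actor that represents a sound packet travelling along precomputed path points, carrying low, mid and high-frequency intensities.
; Each tick it moves by packet velocity, applying inverse-square and exponential air-absorption falloff, and destroys itself when faint or finished.
; At segment ends, gated by both spawn flags, surface materials scale intensities and sufficiently loud packets trigger transmission through the sound system.
; Overlapping a BP_DiffractionEdge reports diffraction to that system when allowed.
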(event Custom|SphereCode
  (bind _packetdata (Variables|Default|GetPacketData))
  (bind _packetdata_2 (Variables|Default|GetPacketData))
  (bind _packetdata_3 (Variables|Default|GetPacketData))
  (bind _returnvalue (Utilities|Array|Length (.pathpoints _packetdata_3)))
  (Variables|Default|SetCurrentLFIntensity (* (Variables|Default|GetStartLFIntensity) (Variables|Default|GetLFFalloff)))
  (Variables|Default|SetCurrentMFIntensity (* (Variables|Default|GetStartMFIntensity) (Variables|Default|GetMFFalloff)))
  (Variables|Default|SetCurrentHFIntensity (* (Variables|Default|GetStartHFIntensity) (Variables|Default|GetHFFalloff)))
  (Variables|Default|SetCurrentIntensity (+ (Variables|Default|GetCurrentLFIntensity) (Variables|Default|GetCurrentMFIntensity) (Variables|Default|GetCurrentHFIntensity)))
  (if (< (Variables|Default|GetCurrentIntensity) 0.01)
    (Actor|DestroyActor)
    (elif (< _returnvalue 2)
      (Actor|DestroyActor)
      (elif (>= (Variables|Default|GetCurrentIndex) (+ _returnvalue 1))
        (Actor|DestroyActor)
        (else
          (Variables|Default|SetStartPos (.pathlocations (Utilities|Array|Get(acopy) (.pathpoints _packetdata_3) (Variables|Default|GetCurrentIndex))))
          (Variables|Default|SetEndPos (.pathlocations (Utilities|Array|Get(acopy) (.pathpoints _packetdata_3) (+ (Variables|Default|GetCurrentIndex) 1))))
          (Variables|Default|SetDirection (Math|Vector|Normalize (- (Variables|Default|GetEndPos) (Variables|Default|GetStartPos))))
          (Variables|Default|SetSegmentLength (Math|Vector|VectorLength (- (Variables|Default|GetEndPos) (Variables|Default|GetStartPos))))
          (bind _output_get (Variables|Default|SetDistanceAlongSegment (+ (Variables|Default|GetDistanceAlongSegment) (* (.velocity (Variables|Default|GetPacketData)) (Utilities|Time|GetWorldDeltaSeconds)))))
          (CallFunction|CalculateFalloff _output_get)
          (Transformation|SetActorLocation (+ (Variables|Default|GetStartPos) (* (Variables|Default|GetDirection) (Variables|Default|GetDistanceAlongSegment))) false false)
          (if (Math|Boolean|ANDBoolean (.canspawntransmission _packetdata) (.canspawndiffraction _packetdata) (>= (Variables|Default|GetDistanceAlongSegment) (Variables|Default|GetSegmentLength)))
            (CallFunction|BounceLogic)
            (if (and (.canspawntransmission _packetdata_2) (> (Variables|Default|GetCurrentIntensity) 1e+01))
              (CallFunction|TransmissionLogic)
              (Default|HandleTransmission (Variables|Default|GetSoundSystemRef) (Variables|Default|GetSphereIndex) (Variables|Default|GetCurrentIndex) (+ (Variables|Default|GetEndPos) (* (Math|Vector|Normalize (Variables|Default|GetDirection)) 10)) (Variables|Default|GetCurrentLFIntensity) (Variables|Default|GetCurrentMFIntensity) (Variables|Default|GetCurrentHFIntensity)))
            (bind _result (Math|Integer|IncrementInt (Variables|Default|GetCurrentIndex))
              (:%20%20
                (if (>= _result (- (Utilities|Array|Length (.pathpoints _packetdata_2)) 1))
                  (Actor|DestroyActor)
                  (else
                    (Variables|Default|SetDistanceAlongSegment 0.0)))))))))))

(event Custom|BounceLogic
  (bind _packetdata (Variables|Default|GetPacketData))
  (bind _currentindex (Variables|Default|GetCurrentIndex))
  (bind _returnvalue (+ _currentindex 1))
  (bind _output (Utilities|Array|Get(acopy) (.pathpoints _packetdata) _returnvalue))
  (Variables|Default|SetStartLFIntensity (* (Variables|Default|GetCurrentLFIntensity) (Utilities|Operators|Subtract 1.0 (.absorptionlf (.physmaterial _output)) (.transmissionlf (.physmaterial _output)))))
  (Variables|Default|SetStartMFIntensity (* (Variables|Default|GetCurrentMFIntensity) (Utilities|Operators|Subtract 1.0 (.absorptionmf (.physmaterial _output)) (.transmissionmf (.physmaterial _output)))))
  (Variables|Default|SetStartHFIntensity (* (Variables|Default|GetCurrentHFIntensity) (Utilities|Operators|Subtract 1.0 (.absorptionhf (.physmaterial _output)) (.transmissionhf (.physmaterial _output)))))
  (Variables|Default|SetCurrentLFIntensity (Variables|Default|GetStartLFIntensity))
  (Variables|Default|SetCurrentMFIntensity (Variables|Default|GetStartMFIntensity))
  (Variables|Default|SetCurrentHFIntensity (Variables|Default|GetStartHFIntensity)))

(event Custom|TransmissionLogic
  (bind _packetdata (Variables|Default|GetPacketData))
  (bind _currentindex (Variables|Default|GetCurrentIndex))
  (bind _returnvalue (+ _currentindex 1))
  (bind _output (Utilities|Array|Get(acopy) (.pathpoints _packetdata) _returnvalue))
  (Variables|Default|SetStartLFIntensity (* (Variables|Default|GetCurrentLFIntensity) (.transmissionlf (.physmaterial _output))))
  (Variables|Default|SetStartMFIntensity (* (Variables|Default|GetCurrentMFIntensity) (.transmissionmf (.physmaterial _output))))
  (Variables|Default|SetStartHFIntensity (* (Variables|Default|GetCurrentHFIntensity) (.transmissionhf (.physmaterial _output))))
  (Variables|Default|SetCurrentLFIntensity (Variables|Default|GetStartLFIntensity))
  (Variables|Default|SetCurrentMFIntensity (Variables|Default|GetStartMFIntensity))
  (Variables|Default|SetCurrentHFIntensity (Variables|Default|GetStartHFIntensity)))

(event Custom|DiffractionLogic
  (Variables|Default|SetStartLFIntensity (* (Variables|Default|GetCurrentLFIntensity) 1.0))
  (Variables|Default|SetStartMFIntensity (* (Variables|Default|GetCurrentMFIntensity) 1.0))
  (Variables|Default|SetStartHFIntensity (* (Variables|Default|GetCurrentHFIntensity) 1.0)))

(event Custom|CalculateFalloff
  (params (Distance :type Float%20%28double-precision%29))
  (bind _returnvalue (/ Distance 1e+02))
  (bind _returnvalue_2 (/ Distance 1e+02))
  (bind _returnvalue_3 (/ Distance 1e+02))
  (bind _returnvalue_4 (Math|Float|Max(Float) _returnvalue_3 1.0))
  (bind _returnvalue_5 (Math|Float|Max(Float) _returnvalue 1.0))
  (bind _returnvalue_6 (Math|Float|Max(Float) _returnvalue_2 1.0))
  (Variables|Default|SetLFFalloff (/ (* (Class|KismetMathLibrary|Exp (* (Variables|Default|GetAirLFCoefficient) -1.0 _returnvalue_4)) 1.0) (Math|Float|Square _returnvalue_4)))
  (Variables|Default|SetMFFalloff (/ (* (Class|KismetMathLibrary|Exp (* (Variables|Default|GetAirMFCoefficient) -1.0 _returnvalue_6)) 1.0) (Math|Float|Square _returnvalue_6)))
  (Variables|Default|SetHFFalloff (/ (* (Class|KismetMathLibrary|Exp (* (Variables|Default|GetAirHFCoefficient) -1.0 _returnvalue_5)) 1.0) (Math|Float|Square _returnvalue_5))))

(event Collision|EventActorBeginOverlap
  (params (OtherActor :type Actor%20Object%20Reference))
  (bind _asbp_diffraction_edge (Utilities|Casting|CastToBP_DiffractionEdge OtherActor))
  (if (.canspawndiffraction (Variables|Default|GetPacketData))
    (CallFunction|DiffractionLogic)
    (Default|HandleDiffraction (Variables|Default|GetSoundSystemRef) (Variables|Default|GetEndPos) (Variables|Default|GetDirection) _asbp_diffraction_edge (Variables|Default|GetCurrentLFIntensity) (Variables|Default|GetCurrentMFIntensity) (Variables|Default|GetCurrentHFIntensity))))

(event EventBeginPlay
  (bind _packetdata (Variables|Default|GetPacketData))
  (Variables|Default|SetSphereIndex (.index _packetdata))
  (Variables|Default|SetStartLFIntensity (.lfintensity _packetdata))
  (Variables|Default|SetStartMFIntensity (.mfintensity _packetdata))
  (Variables|Default|SetStartHFIntensity (.hfintensity _packetdata)))

(event EventTick
  (params (DeltaSeconds :type Float%20%28single-precision%29))
  (CallFunction|SphereCode))

(fn ConstructionScript)